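; Player Blueprint for a Crossy Road-style game that hops in fixed steps forward, left or right.
; Input calls TryMove, which shifts TargetPos, adds and prints score for any direction, then locks movement until a short timer calls EnableCanMove.
; Tick drives the root component toward TargetPos with MoveComponentTo.
; GameOver reloads the current level and has no caller in this Blueprint.
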(event `InputAction|MoveForward`
  (params (Key :type "Key Structure"))
  (:`Pressed`
    (`self.tryMove` (100.0 0.0 0.0))))

(event `InputAction|MoveLeft`
  (params (Key :type "Key Structure"))
  (:`Pressed`
    (`self.tryMove` (0.0 -100.0 0.0))))

(event `InputAction|MoveRight`
  (params (Key :type "Key Structure"))
  (:`Pressed`
    (`self.tryMove` (0.0 100.0 0.0))))

(event `self.ReceiveTick`
  (params (DeltaSeconds :type "Float (single-precision)"))
  (`KismetSystemLibrary.MoveComponentTo` (`self.DefaultSceneRoot`) (`self.targetPos`)))

(fn `enableCanMove`
  (set `self.canMove` true))

(fn `gameOver`
  (bind _returnvalue (`GameplayStatics.GetCurrentLevelName` true))
  (`GameplayStatics.OpenLevel` (`KismetStringLibrary.Conv_StringToName` _returnvalue)))

(fn `tryMove`
  (params (direction :type "Vector Structure"))
  (if (`self.canMove`)
    (set `self.targetPos` (+ direction (`self.targetPos`)))
    (set `self.canMove` false)
    (bind _output_get (set `self.score` (+ (`self.score`) 5)))
    (`KismetSystemLibrary.PrintString` (`KismetStringLibrary.Conv_IntToString` _output_get))
    (`KismetSystemLibrary.K2_SetTimer` null "enableCanMove" 0.3)))

(fn `UserConstructionScript`)